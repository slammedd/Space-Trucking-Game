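; BP_Car1 is a car that moves its static mesh along a spline automatically from BeginPlay.
; The Move_Object timeline has its play rate set from TimeToComplete, and its MoveTrack value is mapped to a distance along the spline.
; Each update sets the mesh's world transform from that point, with fixed height and yaw offsets; location is sampled in world space but rotation in local space.
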(event EventBeginPlay
  (bind _spline (Variables|Default|GetSpline))
  (Components|Timeline|SetPlayRate (Variables|Default|GetMove_Object) (/ 1.0 (Variables|Default|GetTime%20to%20Complete)))
  (bind _move_track (Timeline|Move_Object Play)
    (:Update
      (Transformation|SetWorldTransform (Variables|Default|GetStaticMesh) (Math|Transform|MakeTransform (Math|Vector|MakeVector (.x (Spline|GetLocationatDistanceAlongSpline _spline (Math|Float|Lerp 0.0 (Spline|GetSplineLength (Variables|Default|GetSpline)) _move_track) "World")) (.y (Spline|GetLocationatDistanceAlongSpline _spline (Math|Float|Lerp 0.0 (Spline|GetSplineLength (Variables|Default|GetSpline)) _move_track) "World")) (+ (.z (Spline|GetLocationatDistanceAlongSpline _spline (Math|Float|Lerp 0.0 (Spline|GetSplineLength (Variables|Default|GetSpline)) _move_track) "World")) 75.0)) (Math|Rotator|MakeRotator (.roll (Spline|GetRotationatDistanceAlongSpline _spline (Math|Float|Lerp 0.0 (Spline|GetSplineLength (Variables|Default|GetSpline)) _move_track) "Local")) (.pitch (Spline|GetRotationatDistanceAlongSpline _spline (Math|Float|Lerp 0.0 (Spline|GetSplineLength (Variables|Default|GetSpline)) _move_track) "Local")) (+ (.yaw (Spline|GetRotationatDistanceAlongSpline _spline (Math|Float|Lerp 0.0 (Spline|GetSplineLength (Variables|Default|GetSpline)) _move_track) "Local")) -7e+01)) "1.000000,1.000000,1.000000") false false))))

(fn ConstructionScript)