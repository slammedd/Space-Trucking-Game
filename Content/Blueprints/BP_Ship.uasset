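; BP_Ship is a flyable ship pawn that the player boards, powers up, flies and exits when landed.
; Line traces detect landing and deploy gear, feeding a Landed/Hover/Cruise state that governs FloatingPawnMovement input and tuning.
; Tick interpolates hull rotation, tilt and thruster pivot from input, and scales camera shake with speed.
; Timelines animate power, mode switches and gear alongside Niagara thruster effects, with a zoomable, toggleable free-look camera.
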(event Custom|Thruster%20Power%20Down
  (bind _thruster_l_vfx (Variables|Default|GetThruster%20L%20VFX))
  ;[1 1 1] Power On/Off Effects
  (if (not (Variables|Default|GetSwitching%20Power%20States))
    (if (Variables|Default|GetGrounded)
      (Variables|Default|SetSwitching%20Power%20States true)
      (bind _rotation (Timeline|Thruster%20Off%20Animation ReverseFromEnd)
        (:Update
          (Transformation|SetRelativeRotation (Variables|Default|GetThruster%20Pivot) (Math|Rotator|MakeRotator _rotation 0.0 -9e+01) false false)
          (Utilities|FlowControl|DoOnce false :!label _label
            (:Completed
              (Components|Activation|Deactivate _thruster_l_vfx)
              (Niagara|SpawnSystemAttached "/Game/VFX/Thruster_VFX/Niagara/NS_Thrust_Low.NS_Thrust_Low" _thruster_l_vfx "None" "0, 0, 0" "0, 0, 0" "SnapToTargetIncludingScale" true)
              (Niagara|SpawnSystemAttached "/Game/VFX/Thruster_VFX/Niagara/NS_Thrust_Low.NS_Thrust_Low" (Variables|Default|GetThruster%20R%20VFX) "None" "0, 0, 0" "0, 0, 0" "SnapToTargetIncludingScale" true)
              (Variables|Default|SetEngine%20On false))))
        (:Finished
          (Variables|Default|SetSwitching%20Power%20States false)
          (Variables|Default|SetThruster%20State "NewEnumerator2")
          (goto _label Reset))))))

(event Custom|Rotation%20Control%20Enable%20Timer
  ;[1 1 1] Rotation Control Enable Timer
  (if (not (Variables|Default|GetRot%20Timer%20Fired))
    (Utilities|FlowControl|Delay 0.3)
    (Variables|Default|SetShip%20State "NewEnumerator1")
    (Variables|Default|SetUnlock%20Controls true)
    (Variables|Default|SetRot%20Timer%20Fired true)))

(event Custom|Gear_Down
  ;[1 1 1] Auto Landing Gear
  (Utilities|FlowControl|DoOnce false
    (:Completed
      (bind _location (Timeline|Gear%20Movement%20Reverse ReverseFromEnd)
        (:Update
          (Transformation|SetRelativeLocation (Variables|Default|GetRight%20Gear) (Math|Vector|MakeVector 0.0 0.0 _location) false false)
          (Transformation|SetRelativeLocation (Variables|Default|GetLeft%20Gear) (Math|Vector|MakeVector 0.0 0.0 _location) false false))
        (:Finished
          (Variables|Default|SetGear%20Down true)
          (Utilities|FlowControl|DoOnce false) ; enters at Reset
        )))))

(event Custom|Gear%20Up
  ;[1 1 1] Auto Landing Gear
  (Utilities|FlowControl|DoOnce false
    (:Completed
      (bind _location (Timeline|Gear%20Movement PlayFromStart)
        (:Update
          (Transformation|SetRelativeLocation (Variables|Default|GetRight%20Gear) (Math|Vector|MakeVector 0.0 0.0 _location) false false)
          (Transformation|SetRelativeLocation (Variables|Default|GetLeft%20Gear) (Math|Vector|MakeVector 0.0 0.0 _location) false false))
        (:Finished
          (Variables|Default|SetGear%20Down false)
          (Utilities|FlowControl|DoOnce false) ; enters at Reset
        )))))

(event Custom|Auto%20Level%20Ship
  (bind _auto_level_speed (Variables|Default|GetAuto%20Level%20Speed))
  (bind _ship_rotation_scene_comp (Variables|Default|GetShip%20Rotation%20Scene%20Comp))
  (bind _returnvalue (Transformation|GetWorldRotation _ship_rotation_scene_comp))
  ;[1 1 1] Auto Level
  (Class|PawnMovementComponent|ConsumeInputVector (Variables|Default|GetFloatingPawnMovement))
  (Pawn|SetControlRotation (Pawn|GetController) (Math|Rotator|MakeRotator 0.0 0.0 0.0))
  (Transformation|SetWorldRotation (Variables|Default|GetShip%20Rotation%20Scene%20Comp) (Math|Rotator|MakeRotator (Math|Interpolation|FInterpTo (.roll _returnvalue) 0.0 (stale EventTick DeltaSeconds) _auto_level_speed) (Math|Interpolation|FInterpTo (.pitch _returnvalue) 0.0 (stale EventTick DeltaSeconds) _auto_level_speed) (Math|Interpolation|FInterpTo (.yaw _returnvalue) 0.0 (stale EventTick DeltaSeconds) _auto_level_speed)) false false)
  (Utilities|FlowControl|Delay 2.5)
  (Variables|Default|SetAuto%20Level false))

(event Custom|Cruise%20Mode%20Settings
  (bind _floatingpawnmovement (Variables|Default|GetFloatingPawnMovement))
  ;[1 1 1] Movement Settings
  (Variables|/Script/Engine.FloatingPawnMovement|SetMaxSpeed _floatingpawnmovement 1.5e+04)
  (Variables|/Script/Engine.FloatingPawnMovement|SetAcceleration _floatingpawnmovement 1.5e+03)
  (Variables|/Script/Engine.FloatingPawnMovement|SetDeceleration _floatingpawnmovement 2.5e+02)
  (Variables|/Script/Engine.FloatingPawnMovement|SetTurningBoost _floatingpawnmovement 0.0)
  (Variables|Default|SetShip%20Rotation%20Interp%20Speed 1.0)
  (Variables|Default|SetShip%20Movement%20Tilt%20Amount 4.0)
  (Variables|Default|SetShip%20Tilt%20Interp%20Speed 3.0)
  (Variables|Default|SetThruster%20Movement%20Tilt%20Amount 5.0))

(event Custom|Hover%20Mode%20Settings
  (bind _floatingpawnmovement (Variables|Default|GetFloatingPawnMovement))
  ;[1 1 1] Movement Settings
  (Variables|/Script/Engine.FloatingPawnMovement|SetMaxSpeed _floatingpawnmovement 1.5e+03)
  (Variables|/Script/Engine.FloatingPawnMovement|SetAcceleration _floatingpawnmovement 5e+02)
  (Variables|/Script/Engine.FloatingPawnMovement|SetDeceleration _floatingpawnmovement 5e+02)
  (Variables|/Script/Engine.FloatingPawnMovement|SetTurningBoost _floatingpawnmovement 0.25)
  (Variables|Default|SetShip%20Rotation%20Interp%20Speed 3.0)
  (Variables|Default|SetShip%20Movement%20Tilt%20Amount 4.0)
  (Variables|Default|SetShip%20Tilt%20Interp%20Speed 1.0)
  (Variables|Default|SetThruster%20Movement%20Tilt%20Amount 8.0))

(event Custom|Thrusters%20Crusise%20Mode
  ;[1 1 1] Thruster Modes
  (if (not (Variables|Default|GetIs%20Changing%20Thruster%20Modes))
    (Variables|Default|SetIs%20Changing%20Thruster%20Modes true)
    (Variables|Default|SetUnlock%20Controls false)
    (Variables|Default|SetInterp%20Switch false)
    (bind _rotation (Timeline|Cruise%20Mode%20Thruster PlayFromStart)
      (:Update
        (Transformation|SetRelativeRotation (Variables|Default|GetThruster%20Pivot) (Math|Rotator|MakeRotator _rotation 0.0 -9e+01) false false)
        (Pawn|Input|AddMovementInput (Math|Vector|GetForwardVector (Pawn|GetControlRotation :!class /Script/Engine.Pawn)) 0.3 false))
      (:Finished
        (Variables|Default|SetShip%20State "NewEnumerator2")
        (Variables|Default|SetUnlock%20Controls true)
        (Variables|Default|SetIs%20Changing%20Thruster%20Modes false)
        (Variables|Default|SetInterp%20Switch true)
        (Components|Activation|Deactivate (Variables|Default|GetThruster%20R%20VFX))
        (Niagara|SpawnSystemAttached "/Game/VFX/Thruster_VFX/Niagara/NS_Thrust_Spawn.NS_Thrust_Spawn" (Variables|Default|GetThruster%20R%20VFX) "None" "0, 0, 0" "0, 0, 0" "SnapToTargetIncludingScale" true)
        (Niagara|SpawnSystemAttached "/Game/VFX/Thruster_VFX/Niagara/NS_Thrust_Spawn.NS_Thrust_Spawn" (Variables|Default|GetThruster%20L%20VFX) "None" "0, 0, 0" "0, 0, 0" "SnapToTargetIncludingScale" true)
        (Utilities|FlowControl|Delay 0.2)
        (Class|NiagaraComponent|SetAsset (Variables|Default|GetThruster%20R%20VFX) "/Game/VFX/Thruster_VFX/Niagara/NS_Thrust_Constant.NS_Thrust_Constant" true)
        (Components|Activation|Activate (Variables|Default|GetThruster%20L%20VFX) false)))))

(event Custom|Thrusters%20Hover%20Mode
  ;[1 1 1] Thruster Modes
  (if (not (Variables|Default|GetIs%20Changing%20Thruster%20Modes))
    (Variables|Default|SetIs%20Changing%20Thruster%20Modes true)
    (Variables|Default|SetUnlock%20Controls false)
    (Variables|Default|SetInterp%20Switch false)
    (bind _rotation (Timeline|Timeline_0 PlayFromStart)
      (:Update
        (Transformation|SetRelativeRotation (Variables|Default|GetThruster%20Pivot) (Math|Rotator|MakeRotator _rotation 0.0 -9e+01) false false)
        (Pawn|Input|AddMovementInput (Math|Vector|GetForwardVector (Pawn|GetControlRotation :!class /Script/Engine.Pawn)) 0.3 false))
      (:Finished
        (Variables|Default|SetShip%20State "NewEnumerator1")
        (Variables|Default|SetUnlock%20Controls true)
        (Variables|Default|SetIs%20Changing%20Thruster%20Modes false)
        (Variables|Default|SetInterp%20Switch true)
        (Components|Activation|Deactivate (Variables|Default|GetThruster%20R%20VFX))
        (Niagara|SpawnSystemAttached "/Game/VFX/Thruster_VFX/Niagara/NS_Thrust_Spawn.NS_Thrust_Spawn" (Variables|Default|GetThruster%20R%20VFX) "None" "0, 0, 0" "0, 0, 0" "SnapToTargetIncludingScale" true)
        (Niagara|SpawnSystemAttached "/Game/VFX/Thruster_VFX/Niagara/NS_Thrust_Spawn.NS_Thrust_Spawn" (Variables|Default|GetThruster%20L%20VFX) "None" "0, 0, 0" "0, 0, 0" "SnapToTargetIncludingScale" true)
        (Utilities|FlowControl|Delay 0.2)
        (Class|NiagaraComponent|SetAsset (Variables|Default|GetThruster%20R%20VFX) "/Game/VFX/Thruster_VFX/Niagara/NS_Thrust_Constant_Low.NS_Thrust_Constant_Low" true)
        (Components|Activation|Activate (Variables|Default|GetThruster%20L%20VFX) false)))))

(event EventInteract
  ;[1 1 1] Pilot/Leave Ship
  (Variables|Default|SetPilot (Game|GetPlayerCharacter 0))
  (if (not (Variables|Default|GetIs%20Piloting%20Ship))
    (Collision|SetActorEnableCollision (Variables|Default|GetPilot) false)
    (Pawn|Possess (Game|GetPlayerController 0) self)
    (Variables|Default|SetIs%20Piloting%20Ship true)
    (Variables|Default|SetInterp%20Switch true)))

(event EventTick
  (params (DeltaSeconds :type Float%20%28single-precision%29))
  (bind _returnvalue (Pawn|GetControlRotation :!class /Script/Engine.Pawn))
  (bind _returnvalue_2 (Pawn|GetControlRotation :!class /Script/Engine.Pawn))
  (bind _thruster_pivot (Variables|Default|GetThruster%20Pivot))
  (bind _ship_rotation_scene_comp (Variables|Default|GetShip%20Rotation%20Scene%20Comp))
  (bind _thruster_pivot_2 (Variables|Default|GetThruster%20Pivot))
  (bind _floatingpawnmovement (Variables|Default|GetFloatingPawnMovement))
  (bind _thruster_pivot_3 (Variables|Default|GetThruster%20Pivot))
  (bind _ship_tilt_interp_speed (Variables|Default|GetShip%20Tilt%20Interp%20Speed))
  (bind _ship_scene_comp (Variables|Default|GetShip%20Scene%20Comp))
  (bind _thruster_pivot_4 (Variables|Default|GetThruster%20Pivot))
  (bind _floatingpawnmovement_2 (Variables|Default|GetFloatingPawnMovement))
  (bind _thruster_tilt_interp_speed (Variables|Default|GetThruster%20Tilt%20Interp%20Speed))
  (bind _thruster_pivot_5 (Variables|Default|GetThruster%20Pivot))
  (bind _thruster_pivot_6 (Variables|Default|GetThruster%20Pivot))
  (bind _thruster_tilt_interp_speed_2 (Variables|Default|GetThruster%20Tilt%20Interp%20Speed))
  (bind _returnvalue_3 (Pawn|Components|PawnMovement|GetLastInputVector _floatingpawnmovement_2))
  (bind _returnvalue_4 (Pawn|Components|PawnMovement|GetLastInputVector _floatingpawnmovement))
  (bind _relativerotation (Variables|/Script/Engine.SceneComponent|GetRelativeRotation _thruster_pivot))
  (bind _relativerotation_2 (Variables|/Script/Engine.SceneComponent|GetRelativeRotation _thruster_pivot_4))
  (bind _relativerotation_3 (Variables|/Script/Engine.SceneComponent|GetRelativeRotation _ship_scene_comp))
  (bind _relativerotation_4 (Variables|/Script/Engine.SceneComponent|GetRelativeRotation _thruster_pivot_3))
  (bind _relativerotation_5 (Variables|/Script/Engine.SceneComponent|GetRelativeRotation _thruster_pivot_5))
  (bind _relativerotation_6 (Variables|/Script/Engine.SceneComponent|GetRelativeRotation _thruster_pivot_6))
  (CallFunction|FloorDetection)
  (CallFunction|LandingGearDeployCheck)
  ;[1 1 1] Speed Scaling Camera Shake
  (if (Variables|Default|GetEngine%20On)
    (if (Variables|Default|GetAlt%20Camera)
      (CameraShake|StopAllCameraShakes (Game|GetPlayerCameraManager 0) true)
      (else
        (Class|MatineeCameraShake|StartMatineeCameraShake (Game|GetPlayerCameraManager 0) "/Game/VFX/CS_Ship.CS_Ship_C" (/ (Math|Vector|VectorLength (Transformation|GetVelocity)) (* (Variables|Default|GetCamera%20Shake%20Speed%20Scale%20Factor) 1e+02)) "CameraLocal" "0, 0, 0")))
    (switch Utilities|FlowControl|Switch|SwitchonE_Ship_States (Variables|Default|GetShip%20State)
      (:NewEnumerator1
        (CallFunction|LandingGearDeployCheck))
      (:NewEnumerator2
        (Pawn|Input|AddMovementInput (Math|Vector|GetForwardVector (Pawn|GetControlRotation :!class /Script/Engine.Pawn)) 1.0 true)
        (if (Variables|Default|GetAuto%20Level)
          (CallFunction|AutoLevelShip))))
    ;[1 1 1] Hover Movement
    (if (Variables|Default|GetInterp%20Switch)
      (Transformation|SetWorldRotation _ship_rotation_scene_comp (Math|Interpolation|RInterpTo (Transformation|GetWorldRotation _ship_rotation_scene_comp) (Pawn|GetControlRotation :!class /Script/Engine.Pawn) DeltaSeconds (Variables|Default|GetShip%20Rotation%20Interp%20Speed)) false false)
      (Transformation|SetRelativeRotation (Variables|Default|GetShip%20Scene%20Comp) (Math|Rotator|MakeRotator (Math|Interpolation|FInterpTo (.roll _relativerotation_3) (* (Math|Vector|DotProduct _returnvalue_4 (Math|Vector|GetRightVector _returnvalue)) (Variables|Default|GetShip%20Movement%20Tilt%20Amount)) DeltaSeconds _ship_tilt_interp_speed) (Math|Interpolation|FInterpTo (.pitch _relativerotation_3) (* (Math|Vector|DotProduct _returnvalue_4 (Math|Vector|GetForwardVector _returnvalue)) (* (Variables|Default|GetShip%20Movement%20Tilt%20Amount) -1.0)) DeltaSeconds _ship_tilt_interp_speed) 0.0) false false)
      ;[1 1 1] Thruster Rotation
      (switch Utilities|FlowControl|Switch|SwitchonE_Ship_States (Variables|Default|GetShip%20State)
        (:NewEnumerator1
          (Transformation|SetRelativeRotation (Variables|Default|GetThruster%20Pivot) (Math|Rotator|MakeRotator (Math|Interpolation|FInterpTo (.roll _relativerotation_4) (+ (* (Math|Vector|DotProduct _returnvalue_3 (Math|Vector|GetForwardVector _returnvalue_2)) (Variables|Default|GetThruster%20Movement%20Tilt%20Amount)) -75.0) DeltaSeconds _thruster_tilt_interp_speed) (Math|Interpolation|FInterpTo (.pitch _relativerotation_4) (* (Math|Vector|DotProduct (Math|Vector|GetRightVector _returnvalue_2) _returnvalue_3) (Variables|Default|GetThruster%20Movement%20Tilt%20Amount)) DeltaSeconds _thruster_tilt_interp_speed) -9e+01) false false))
        (:NewEnumerator2
          ;[1 1 1] Cruise Mode Thrusters
          (if (not (Variables|Default|GetAlt%20Camera))
            (Transformation|SetRelativeRotation _thruster_pivot_2 (Math|Rotator|MakeRotator (Math|Interpolation|FInterpTo (.roll _relativerotation_2) (+ (Variables|Default|GetU/D%20Gamepad) (.roll _relativerotation_2)) DeltaSeconds _thruster_tilt_interp_speed_2) 0.0 (Math|Interpolation|FInterpTo (.yaw _relativerotation_2) (+ (Variables|Default|GetR/L%20Gamepad) (.yaw _relativerotation_2)) DeltaSeconds (Variables|Default|GetThruster%20Tilt%20Interp%20Speed))) false false)
            (Transformation|SetRelativeRotation _thruster_pivot_2 (Math|Rotator|MakeRotator (Math|Interpolation|FInterpTo (.roll _relativerotation_2) (+ (Variables|Default|GetU/D%20Mouse) (.roll _relativerotation_2)) DeltaSeconds _thruster_tilt_interp_speed_2) 0.0 (Math|Interpolation|FInterpTo (.yaw _relativerotation_2) (+ (Variables|Default|GetR/L%20Mouse) (.yaw _relativerotation_2)) DeltaSeconds (Variables|Default|GetThruster%20Tilt%20Interp%20Speed))) false false)
            (Transformation|SetRelativeRotation _thruster_pivot_5 (Math|Rotator|MakeRotator (Math|Float|Clamp(Float) (.roll _relativerotation_5) -2e+01 2e+01) 0.0 (Math|Float|Clamp(Float) (.yaw _relativerotation_5) -1.1e+02 -7e+01)) false false)
            (if (and (== (Variables|Default|GetU/D%20Gamepad) 0.0) (== (Variables|Default|GetU/D%20Mouse) 0.0))
              (Transformation|SetRelativeRotation _thruster_pivot (Math|Rotator|MakeRotator (Math|Interpolation|FInterpTo (.roll _relativerotation) 0.0 DeltaSeconds (Variables|Default|GetThruster%20Tilt%20Interp%20Speed)) 0.0 (.yaw _relativerotation)) false false))
            (if (and (== (Variables|Default|GetR/L%20Gamepad) 0.0) (== (Variables|Default|GetR/L%20Mouse) 0.0))
              (Transformation|SetRelativeRotation _thruster_pivot_6 (Math|Rotator|MakeRotator (.roll _relativerotation_6) 0.0 (Math|Interpolation|FInterpTo (.yaw _relativerotation_6) -9e+01 DeltaSeconds (Variables|Default|GetThruster%20Tilt%20Interp%20Speed))) false false))))))))

(event Input|ActionEvents|InputActionInteract
  (params (Key :type Key%20Structure :default "None"))
  (bind _pilot (Variables|Default|GetPilot))
  (bind _arrow (Variables|Default|GetArrow))
  ;[1 1 1] Pilot/Leave Ship
  (:Pressed
    (if (Variables|Default|GetIs%20Piloting%20Ship)
      (if (not (Variables|Default|GetSwitching%20Power%20States))
        (switch Utilities|FlowControl|Switch|SwitchonE_Ship_States (Variables|Default|GetShip%20State)
          (:NewEnumerator3
            (CallFunction|ThrusterPowerDown)
            (Transformation|SetActorTransform _pilot (Math|Transform|MakeTransform (.location (Transformation|GetWorldTransform _arrow)) (Variables|/Script/Engine.SceneComponent|GetRelativeRotation _arrow) "1.000000,1.000000,1.000000"))
            (Collision|SetActorEnableCollision (Variables|Default|GetPilot) true)
            (Pawn|Possess (Game|GetPlayerController 0) _pilot)
            (Variables|Default|SetIs%20Piloting%20Ship false)
            (Variables|Default|SetInterp%20Switch false)))))))

(event Input|ActionEvents|InputActionAltCamera
  (params (Key :type Key%20Structure :default "None"))
  (bind _springarm (Variables|Default|GetSpringArm))
  ;[1 1 1] Freelook Mode
  (:Pressed
    (switch Utilities|FlowControl|Switch|SwitchonE_Ship_States (Variables|Default|GetShip%20State)
      (:NewEnumerator1
        _)
      (:NewEnumerator2
        _))
    (if (Variables|Default|GetAlt%20Camera)
      (Variables|Default|SetAlt%20Camera false)
      (Variables|/Script/Engine.SpringArmComponent|SetbUsePawnControlRotation _springarm true)
      (else
        (Variables|Default|SetAlt%20Camera true)
        (Variables|/Script/Engine.SpringArmComponent|SetbUsePawnControlRotation _springarm false)))))

(event Input|ActionEvents|InputActionAction
  (params (Key :type Key%20Structure :default "None"))
  ;[1 1 1] Power On/Off Effects
  (:Pressed
    (if (not (Variables|Default|GetSwitching%20Power%20States))
      (if (Variables|Default|GetEngine%20On)
        (CallFunction|ThrusterPowerDown)
        (else
          (Variables|Default|SetSwitching%20Power%20States true)
          (bind _rotation (Timeline|Thruster%20On%20Animation PlayFromStart)
            (:Update
              (Transformation|SetRelativeRotation (Variables|Default|GetThruster%20Pivot) (Math|Rotator|MakeRotator _rotation 0.0 -9e+01) false false))
            (:Finished
              (Variables|Default|SetSwitching%20Power%20States false)
              (Variables|Default|SetThruster%20State "NewEnumerator0")
              (Niagara|SpawnSystemAttached "/Game/VFX/Thruster_VFX/Niagara/NS_Thrust_Low.NS_Thrust_Low" (Variables|Default|GetThruster%20R%20VFX) "None" "0, 0, 0" "0, 0, 0" "SnapToTargetIncludingScale" true)
              (Niagara|SpawnSystemAttached "/Game/VFX/Thruster_VFX/Niagara/NS_Thrust_Low.NS_Thrust_Low" (Variables|Default|GetThruster%20L%20VFX) "None" "0, 0, 0" "0, 0, 0" "SnapToTargetIncludingScale" true)
              (Utilities|FlowControl|Delay 0.4)
              (Components|Activation|Activate (Variables|Default|GetThruster%20L%20VFX) false)
              (Variables|Default|SetEngine%20On true))))))))

(event Input|ActionEvents|InputActionToggleMode
  (params (Key :type Key%20Structure :default "None"))
  ;[1 1 1] Toggle Ship Mode
  (:Pressed
    (switch Utilities|FlowControl|Switch|SwitchonE_Ship_States (Variables|Default|GetShip%20State)
      (:NewEnumerator1
        (CallFunction|CruiseModeSettings)
        (CallFunction|ThrustersCrusiseMode))
      (:NewEnumerator2
        (CallFunction|HoverModeSettings)
        (CallFunction|ThrustersHoverMode)
        (Variables|Default|SetAuto%20Level true)))))

(event Input|AxisEvents|InputAxisLookUp/DownGamepad
  (params (AxisValue :type Float%20%28single-precision%29))
  ;[1 1 1] Freelook Mode
  (if (Variables|Default|GetAlt%20Camera)
    (Transformation|AddRelativeRotation (Variables|Default|GetSpringArm) (Math|Rotator|MakeRotator 0.0 AxisValue 0.0) false false)))

(event Input|AxisEvents|InputAxisLookUp/DownMouse
  (params (AxisValue :type Float%20%28single-precision%29))
  ;[1 1 1] Freelook Mode
  (if (Variables|Default|GetAlt%20Camera)
    (Transformation|AddRelativeRotation (Variables|Default|GetSpringArm) (Math|Rotator|MakeRotator 0.0 AxisValue 0.0) false false)))

(event Input|AxisEvents|InputAxisTurnRight/LeftGamepad
  (params (AxisValue :type Float%20%28single-precision%29))
  (bind _x_look_sensitivy (Variables|Default|GetX%20Look%20Sensitivy))
  (bind _returnvalue (* AxisValue _x_look_sensitivy))
  ;[1 1 1] Hover Movement
  (Variables|Default|SetR/L%20Gamepad AxisValue)
  (switch Utilities|FlowControl|Switch|SwitchonE_Ship_States (Variables|Default|GetShip%20State)
    (:NewEnumerator1
      _)
    (:NewEnumerator2
      _))
  (if (Variables|Default|GetAlt%20Camera)
    ;[1 1 1] Freelook Mode
    (Transformation|AddRelativeRotation (Variables|Default|GetSpringArm) (Math|Rotator|MakeRotator 0.0 0.0 _returnvalue) false false)
    (elif (Variables|Default|GetUnlock%20Controls)
      (Pawn|Input|AddControllerYawInput _returnvalue))))

(event Input|AxisEvents|InputAxisTurnRight/LeftMouse
  (params (AxisValue :type Float%20%28single-precision%29))
  (bind _x_look_sensitivy (Variables|Default|GetX%20Look%20Sensitivy))
  (bind _returnvalue (* AxisValue _x_look_sensitivy))
  ;[1 1 1] Hover Movement
  (Variables|Default|SetR/L%20Mouse AxisValue)
  (switch Utilities|FlowControl|Switch|SwitchonE_Ship_States (Variables|Default|GetShip%20State)
    (:NewEnumerator1
      _)
    (:NewEnumerator2
      _))
  (if (Variables|Default|GetAlt%20Camera)
    ;[1 1 1] Freelook Mode
    (Transformation|AddRelativeRotation (Variables|Default|GetSpringArm) (Math|Rotator|MakeRotator 0.0 0.0 _returnvalue) false false)
    (elif (Variables|Default|GetUnlock%20Controls)
      (Pawn|Input|AddControllerYawInput _returnvalue))))

(event Input|AxisEvents|InputAxisZoomCamera
  (params (AxisValue :type Float%20%28single-precision%29))
  ;[1 1 1] Camera Zoom
  (Variables|/Script/Engine.SpringArmComponent|SetTargetArmLength (Variables|Default|GetSpringArm) (Math|Float|Clamp(Float) (+ (* AxisValue -15.0) (Variables|/Script/Engine.SpringArmComponent|GetTargetArmLength (Variables|Default|GetSpringArm))) 2.25e+03 3e+04)))

(event Input|AxisEvents|InputAxisMoveForward/Backward
  (params (AxisValue :type Float%20%28single-precision%29))
  (bind _returnvalue (Pawn|GetControlRotation :!class /Script/Engine.Pawn))
  (bind _returnvalue_2 (Math|Float|Clamp(Float) AxisValue -0.5 0.0))
  (bind _returnvalue_3 (Math|Vector|GetForwardVector _returnvalue))
  ;[1 1 1] Hover Movement
  (switch Utilities|FlowControl|Switch|SwitchonE_Ship_States (Variables|Default|GetShip%20State)
    (:NewEnumerator1
      (Pawn|Input|AddMovementInput (Math|Vector|GetForwardVector (Pawn|GetControlRotation :!class /Script/Engine.Pawn)) AxisValue false))
    (:NewEnumerator2
      (if (>= _returnvalue_2 0.0)
        (Pawn|Input|AddMovementInput _returnvalue_3 1.0 false)
        (else
          (Pawn|Input|AddMovementInput _returnvalue_3 _returnvalue_2 false))))))

(event Input|AxisEvents|InputAxisMoveRight/Left
  (params (AxisValue :type Float%20%28single-precision%29))
  ;[1 1 1] Hover Movement
  (switch Utilities|FlowControl|Switch|SwitchonE_Ship_States (Variables|Default|GetShip%20State)
    (:NewEnumerator1
      (Pawn|Input|AddMovementInput (Math|Vector|GetRightVector (Pawn|GetControlRotation :!class /Script/Engine.Pawn)) AxisValue false))))

(event Input|AxisEvents|InputAxisMoveUp
  (params (AxisValue :type Float%20%28single-precision%29))
  ;[1 1 1] Hover Movement
  (if (Variables|Default|GetEngine%20On)
    (Pawn|Input|AddMovementInput (Math|Vector|GetUpVector (Pawn|GetControlRotation :!class /Script/Engine.Pawn)) AxisValue false)))

(event Input|AxisEvents|InputAxisLookUp/DownGamepad
  (params (AxisValue :type Float%20%28single-precision%29))
  (bind _y_look_sensitivity (Variables|Default|GetY%20Look%20Sensitivity))
  (bind _returnvalue (* AxisValue _y_look_sensitivity))
  ;[1 1 1] Hover Movement
  (Variables|Default|SetU/D%20Gamepad AxisValue)
  (switch Utilities|FlowControl|Switch|SwitchonE_Ship_States (Variables|Default|GetShip%20State)
    (:NewEnumerator2
      (if (Variables|Default|GetUnlock%20Controls)
        (if (Variables|Default|GetAlt%20Camera)
          (Transformation|AddRelativeRotation (Variables|Default|GetSpringArm) (Math|Rotator|MakeRotator _returnvalue 0.0 0.0) false false)
          (else
            (Pawn|Input|AddControllerPitchInput _returnvalue)))))))

(event Input|AxisEvents|InputAxisLookUp/DownMouse
  (params (AxisValue :type Float%20%28single-precision%29))
  (bind _y_look_sensitivity (Variables|Default|GetY%20Look%20Sensitivity))
  (bind _returnvalue (* AxisValue _y_look_sensitivity))
  ;[1 1 1] Hover Movement
  (Variables|Default|SetU/D%20Mouse AxisValue)
  (switch Utilities|FlowControl|Switch|SwitchonE_Ship_States (Variables|Default|GetShip%20State)
    (:NewEnumerator2
      (if (Variables|Default|GetUnlock%20Controls)
        (if (Variables|Default|GetAlt%20Camera)
          (Transformation|AddRelativeRotation (Variables|Default|GetSpringArm) (Math|Rotator|MakeRotator _returnvalue 0.0 0.0) false false)
          (else
            (Pawn|Input|AddControllerPitchInput _returnvalue)))))))

(fn ConstructionScript)

(fn FloorDetection
  (bind _ground_check_point_l (Variables|Default|GetGround%20Check%20Point%20L))
  (bind _ground_check_point_r (Variables|Default|GetGround%20Check%20Point%20R))
  (bind _returnvalue (Transformation|GetWorldLocation _ground_check_point_r))
  (bind _returnvalue_2 (Transformation|GetWorldLocation _ground_check_point_l))
  (bind _returnvalue_3 (Collision|LineTraceByChannel _returnvalue_2 (+ _returnvalue_2 "0,0,-10.000000") "TraceTypeQuery1" false 0 "None"))
  (bind _returnvalue_4 (Collision|LineTraceByChannel _returnvalue (+ _returnvalue "0,0,-10.000000") "TraceTypeQuery1" false 0 "None"))
  (if (and _returnvalue_4 _returnvalue_3)
    (Variables|Default|SetGrounded true)
    (Variables|Default|SetShip%20State "NewEnumerator3")
    (Variables|Default|SetUnlock%20Controls false)
    (Variables|Default|SetRot%20Timer%20Fired false)
    (CallFunction|HoverModeSettings)
    (else
      (Variables|Default|SetGrounded false)
      (if (Variables|Default|GetEngine%20On)
        (CallFunction|RotationControlEnableTimer)))))

(fn LandingGearDeployCheck
  (bind _body (Variables|Default|GetBody))
  (bind _returnvalue (Transformation|GetWorldLocation _body))
  (bind _returnvalue_2 (Collision|LineTraceByChannel _returnvalue (+ _returnvalue "0,0,-2000.000000") "TraceTypeQuery1" false 0 "None" true "(R=1.000000,G=0.000000,B=0.872540,A=1.000000)"))
  (if _returnvalue_2
    (Variables|Default|SetGround%20In%20Range true)
    (switch Utilities|FlowControl|Switch|SwitchonE_Ship_States (Variables|Default|GetShip%20State)
      (:NewEnumerator1
        (if (not (Variables|Default|GetGear%20Down))
          (CallFunction|GearDown))))
    (else
      (Variables|Default|SetGround%20In%20Range false)
      (switch Utilities|FlowControl|Switch|SwitchonE_Ship_States (Variables|Default|GetShip%20State)
        (:NewEnumerator1
          (if (Variables|Default|GetGear%20Down)
            (CallFunction|GearUp)))))))